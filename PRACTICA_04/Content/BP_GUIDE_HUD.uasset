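; BP_GUIDE_HUD is a HUD Blueprint that draws the game's on-screen status text.
; On BeginPlay it casts the game mode to BP_GUIDE_GAMEMODE and caches it.
; Each DrawHUD call reads Score, Level and Time from that game mode and draws them as canvas text at fixed positions along the top of the screen.
; When the GameOver flag is set, it also draws "GAME OVER" and "Press Enter" prompts in red.
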(event EventBeginPlay
  (bind _asbp_guide_gamemode (Utilities|Casting|CastToBP_GUIDE_GAMEMODE (Game|GetGameMode)))
  (Variables|Default|SetMy_guide_GameMode _asbp_guide_gamemode))

(event EventDrawHUD
  (params (SizeX :type Integer) (SizeY :type Integer))
  (HUD|DrawText (Utilities|String|BuildString(Integer) "Score: " "" (Variables|/Game/BP_GUIDE_GAMEMODE.BP_GUIDE_GAMEMODE_C|GetScore (Variables|Default|GetMy_guide_GameMode))) "(R=0.956863,G=1.000000,B=0.101961,A=1.000000)" 1e+01 1e+01 0 3.0 false)
  (HUD|DrawText (Utilities|String|BuildString(Integer) "Player Level:" "" (Variables|/Game/BP_GUIDE_GAMEMODE.BP_GUIDE_GAMEMODE_C|GetLevel (Variables|Default|GetMy_guide_GameMode))) "(R=0.004497,G=0.000000,B=0.670000,A=1.000000)" 5.5e+02 1e+01 0 3.0 false)
  (HUD|DrawText (Utilities|String|BuildString(Integer) "Time:" "" (Variables|/Game/BP_GUIDE_GAMEMODE.BP_GUIDE_GAMEMODE_C|GetTime (Variables|Default|GetMy_guide_GameMode))) "(R=0,G=0,B=0,A=1)" 3e+02 1e+01 0 3.0 false)
  (if (Variables|/Game/BP_GUIDE_GAMEMODE.BP_GUIDE_GAMEMODE_C|GetGameOver (Variables|Default|GetMy_guide_GameMode))
    (HUD|DrawText "GAME OVER" "(R=0.470000,G=0.000000,B=0.000000,A=1.000000)" 4e+02 2e+02 0 3.0 false)
    (HUD|DrawText "Press Enter" "(R=0.750000,G=0.000000,B=0.000000,A=1.000000)" 4e+02 4e+02 0 3.0 false)))

(fn ConstructionScript)