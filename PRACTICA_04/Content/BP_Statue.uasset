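; BP_Statue is a collectible statue that jumps to random spots within a fixed area until the player touches it.
; InitStatue teleports it, then re-arms a timer by function name to repeat, with a delay that shrinks as the game mode's Level rises.
; Player overlap, unless the game is over, notifies BP_GUIDE_GAMEMODE, destroys the statue and spawns a replacement that relocates itself on BeginPlay.
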(event EventBeginPlay
  (bind _asbp_guide_gamemode (Utilities|Casting|CastToBP_GUIDE_GAMEMODE (Game|GetGameMode)))
  (Variables|Default|SetMy%20Guide%20Game%20Mode _asbp_guide_gamemode)
  (CallFunction|InitStatue))

(event Collision|EventActorBeginOverlap
  (params (OtherActor :type Actor%20Object%20Reference))
  (if (and (== OtherActor (Game|GetPlayerCharacter 0)) (not (Variables|/Game/BP_GUIDE_GAMEMODE.BP_GUIDE_GAMEMODE_C|GetGameOver (Variables|Default|GetMy%20Guide%20Game%20Mode))))
    (Default|StatueCollected (Variables|Default|GetMy%20Guide%20Game%20Mode))
    (Actor|DestroyActor)
    (Game|SpawnActorfromClass "BP_Statue_C" (Transformation|GetActorTransform) "Undefined" 0 0)))

(event EventTick
  (params (DeltaSeconds :type Float%20%28single-precision%29)))

(fn ConstructionScript)

(fn InitStatue
  (Transformation|Teleport (Math|Vector|MakeVector (Math|Random|RandomFloatinRange 4e+02 2.5e+03) (Math|Random|RandomFloatinRange 4e+02 3.5e+03) 0.0) "0, 0, 0")
  (Utilities|Time|SetTimerbyFunctionName 0 "Init Statue" (Math|Conversions|ToFloat(Integer) (- 6 (Variables|/Game/BP_GUIDE_GAMEMODE.BP_GUIDE_GAMEMODE_C|GetLevel (Variables|Default|GetMy%20Guide%20Game%20Mode))))))